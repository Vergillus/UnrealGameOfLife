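; GOFManager is a Game of Life manager actor that, as wired, only enables player input and shows the mouse cursor at BeginPlay.
; Tick is empty, and the delayed GameOfLife call and left-click test are disconnected.
; Unconnected debug prints show mouse positions and convert the deprojected cursor, relative to the actor, into a cell index using MapWidth, MapDepth and 100-unit cells.
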(event `self.ReceiveBeginPlay`
  (bind _returnvalue (`GameplayStatics.GetPlayerController` 0))
  (`self.EnableInput` _returnvalue)
  (set `PlayerController.bShowMouseCursor` true _returnvalue))

(event `self.ReceiveTick`
  (params (DeltaSeconds :type "Float (single-precision)")))

(fn `UserConstructionScript`)